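; Player controller that detects which actor the player clicks under the cursor and prints its display name.
; BeginPlay runs SetupInput, which adds the IMC_General Enhanced Input mapping context.
; IA_Click calls GetItemClicked, a complex cursor trace on TraceTypeQuery3 that returns a hit flag and the actor.
; The click handler prints the result without checking the hit flag.
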(event `self.ReceiveBeginPlay`
  (`self.SetupInput`))

(event `EnhancedInput|/Game/IA_Click`
  (params (ActionValue :type Boolean) (ElapsedSeconds :type "Float (double-precision)") (TriggeredSeconds :type "Float (double-precision)") (InputAction :type "InputAction Object Reference" :default "/Game/IA_Click.IA_Click"))
  (:`Triggered`
    (bind (_bfound _clickedactor) (`self.GetItemClicked`))
    (`KismetSystemLibrary.PrintString` (`KismetSystemLibrary.GetDisplayName` _clickedactor))))

(event `EnhancedInput|/Game/IA_Touch`
  (params (ActionValue :type Boolean) (ElapsedSeconds :type "Float (double-precision)") (TriggeredSeconds :type "Float (double-precision)") (InputAction :type "InputAction Object Reference" :default "/Game/IA_Touch.IA_Touch")))

(fn `GetItemClicked`
  (returns (bFound :type Boolean) (ClickedActor :type "Actor Object Reference"))
  (bind (_bblockinghit _binitialoverlap _time _distance _location _impactpoint _normal _impactnormal _physmat _hitactor) (`GameplayStatics.BreakHitResult` (`self.GetHitResultUnderCursorByChannel` "TraceTypeQuery3")))
  (return _bblockinghit _hitactor))

(fn `SetupInput`
  (bind _returnvalue (subsystem `EnhancedInputLocalPlayerSubsystem`))
  (`/Engine/EditorBlueprintResources/StandardMacros.IsValid` _returnvalue
    (:`Is Valid`
      (`EnhancedInputSubsystemInterface.AddMappingContext` _returnvalue "/Game/IMC_General.IMC_General" 0 (struct)))))

(fn `UserConstructionScript`)