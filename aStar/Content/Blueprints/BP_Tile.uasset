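; BP_Tile is a grid tile actor that places itself within the layout of its owning BP_TileGenerator.
; Initalize attaches the tile to its owner, then sets its relative location from its Column and Row, offset against half the generator's grid dimensions to center the grid on it.
; Spacing comes from the Tile component's bounds, so tiles sit edge to edge on a flat plane.
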(fn `Initalize`
  (bind _returnvalue (`self.GetOwner`))
  (`/Engine/EditorBlueprintResources/StandardMacros.IsValid` _returnvalue
    (:`Is Valid`
      (`self.K2_AttachToActor` _returnvalue "None" "SnapToTarget" "SnapToTarget" "KeepRelative")
      (bind _asbp_tile_generator (cast `/Game/Blueprints/BP_TileGenerator` _returnvalue))
      (`self.K2_SetActorRelativeLocation` (`KismetMathLibrary.MakeVector` (* (.x (* (`.BoxExtent` (`KismetSystemLibrary.GetComponentBounds` (`self.Tile`))) (2.0 2.0 0.0))) (- (/ (`/Game/Blueprints/BP_TileGenerator.Columns` _asbp_tile_generator) 2) (`self.Column`))) (* (.y (* (`.BoxExtent` (`KismetSystemLibrary.GetComponentBounds` (`self.Tile`))) (2.0 2.0 0.0))) (- (/ (`/Game/Blueprints/BP_TileGenerator.Rows` _asbp_tile_generator) 2) (`self.Row`))))))))

(fn `UserConstructionScript`)